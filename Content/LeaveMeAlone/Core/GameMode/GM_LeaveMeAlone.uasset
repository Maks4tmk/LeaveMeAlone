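; GM_LeaveMeAlone is the game mode that runs a countdown and ends the game in a loss when time runs out.
; A looping one-second timer started on BeginPlay decrements GameTime.
; At zero it clears the timer, pauses the game, shows the WBP_Lose widget with UI-only input and enables the mouse cursor on PC_LeaveMeAlone.
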(event Custom|CustomEvent
  (bind _output_get (Variables|Default|SetGame%20Time (- (Variables|Default|GetGame%20Time) 1)))
  (if (== _output_get 0)
    (Utilities|Time|ClearandInvalidateTimerbyHandle (Variables|Default|GetTimer))
    (Game|SetGamePaused true)
    (bind _returnvalue (UserInterface|CreateWidget "/Game/LeaveMeAlone/Widgets/UI/WBP_Lose.WBP_Lose_C"))
    (bind _output_get_2 (Variables|Default|SetLose _returnvalue))
    (UserInterface|Viewport|AddtoViewport _output_get_2 0)
    (Input|SetInputModeUIOnly (Game|GetPlayerController 0) _returnvalue "DoNotLock" false)
    (bind _returnvalue_2 (Actor|GetActorOfClass "/Game/LeaveMeAlone/Core/Controller/PC_LeaveMeAlone.PC_LeaveMeAlone_C"))
    (Variables|/Script/Engine.PlayerController|SetbShowMouseCursor _returnvalue_2 true)))

(event EventBeginPlay
  (bind _returnvalue (Utilities|Time|SetTimerbyEvent (delegate Custom|CustomEvent) 1.0 true))
  (Variables|Default|SetTimer _returnvalue))

(event EventTick
  (params (DeltaSeconds :type Float%20%28single-precision%29)))

(fn ConstructionScript)