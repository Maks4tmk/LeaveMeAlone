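; Player controller for LeaveMeAlone that opens the pause menu when the Pause input is pressed.
; An OnPause flag guards the handler, which stops fire on the first LMABaseWeapon found in the world and pauses the game.
; It then creates and shows WBP_Pause, switches to UI-only input and shows the cursor.
; Resuming and resetting the flag are not handled in this graph.
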(event EventBeginPlay)

(event EventTick
  (params (DeltaSeconds :type Float%20%28single-precision%29)))

(event Input|ActionEvents|InputActionPause
  (params (Key :type Key%20Structure :default "None"))
  (:Pressed
    (if (not (Variables|Default|GetOnPause))
      (Variables|Default|SetOnPause true)
      (bind _returnvalue (Actor|GetActorOfClass "/Script/LeaveMeAlone.LMABaseWeapon"))
      (Class|LMABaseWeapon|StopFire _returnvalue)
      (Game|SetGamePaused true)
      (bind _returnvalue_2 (UserInterface|CreateWidget "/Game/LeaveMeAlone/Widgets/UI/WBP_Pause.WBP_Pause_C"))
      (bind _output_get (Variables|Default|SetPauseWidget _returnvalue_2))
      (UserInterface|Viewport|AddtoViewport _output_get 0)
      (Input|SetInputModeUIOnly (Game|GetPlayerController 0) _output_get "DoNotLock" false)
      (Variables|Default|SetbShowMouseCursor true))))

(fn ConstructionScript)